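; Base actor for enemy equipment, serving as weapon or armor, with mesh and stats loaded from DT_Euipment by ID.
; ChangeAttackState toggles an attack window in which mesh overlaps deal DT_AbilityDamage damage scaled by BaseAttack.
; Hits on the equipment forward to its Master, with element amount scaled by resistance / (resistance + ElementConstant).
; OnDead enables mesh physics; special effect, tick and most other functions are empty stubs.
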(event `self.ReceiveBeginPlay`
  (`self.Init`))

(event `self.ReceiveTick`
  (params (DeltaSeconds :type "Float (single-precision)"))
  (`self.Equipment Tick` DeltaSeconds))

(event `/Game/EquipmentForEnemy/BPI_Equipment.Change Attack State`
  (params (Ability :type "/Game/Enemy/Enum/E_HumanAbilities Enum" :default "NewEnumerator0"))
  (`/Engine/EditorBlueprintResources/StandardMacros.FlipFlop`
    (:`A`
      (set `self.Attack?` true)
      (set `self.Cur Ability` Ability))
    (:`B`
      (set `self.Attack?` false))))

(event `self.StaticMesh.OnComponentBeginOverlap`
  (params (OverlappedComponent :type "PrimitiveComponent Object Reference") (OtherActor :type "Actor Object Reference") (OtherComp :type "PrimitiveComponent Object Reference") (OtherBodyIndex :type Integer) (bFromSweep :type Boolean) (SweepResult :type "HitResult Structure (by ref)"))
  (if (`self.Attack?`)
    (bind _returnvalue (`|GetDataTableRow` "/Game/Enemy/DT_AbilityDamage.DT_AbilityDamage" (`|GetEnumeratorName` (`self.Cur Ability`)))
      (:`then`
        (bind (_damageamount _damagetype _damageresponse _shoulddamageinvincible _canbeblocked _canbeparried _shouldforceinterrupt _element _canaddbuff_ _elementamount _elementdamageamount _buff _instigator _location) (break `/Game/Enemy/DamageSystem/S_DamageInfomation` _returnvalue))
        (message `/Game/Enemy/DamageSystem/BPI_Damagable.Take Damage` OtherActor (make `/Game/Enemy/DamageSystem/S_DamageInfomation` (* _damageamount (`.BaseAttack_15_747FB1244D31DC950D6B8AA85A9D6FB6` (break `/Game/EquipmentForEnemy/S_Equipment` (`self.Equipment`)))) _damagetype _damageresponse _shoulddamageinvincible _canbeblocked _canbeparried _shouldforceinterrupt _element _canaddbuff_ _elementamount _elementdamageamount _buff _instigator _location))))))

(fn `Element Amount Decrease`
  (params (Key :type "/Game/Enemy/DamageSystem/E_ElementType Enum (by ref)") (A :type "Float (double-precision)"))
  (returns (ReturnValue :type "Float (double-precision)"))
  (bind _value (`BlueprintMapLibrary.Map_Find` (`.BaseElementResistance_37_C3A7779C48B6D176E6D7B18DD840D915` (break `/Game/EquipmentForEnemy/S_Equipment` (`self.Equipment`))) Key))
  (return (* A (/ _value (+ _value (`self.Element Constant`))))))

(fn `Equipment Special Effect`)

(fn `Equipment Tick`
  (params (`Delta Time` :type "Float (double-precision)")))

(fn `Get Buff Handler`
  (returns (`AC_Buff Handler` :type "/Game/BUFF/AC_BuffHandler Object Reference"))
  (return null))

(fn `Get Current Health`
  (returns (Health :type "Float (double-precision)"))
  (return 0.0))

(fn `Get Current Toughness`
  (returns (Value :type "Float (double-precision)"))
  (return 0.0))

(fn `Get Max Health`
  (returns (`Max Health` :type "Float (double-precision)"))
  (return 0.0))

(fn `Get Max Toughness`
  (returns (Value :type "Float (double-precision)"))
  (return 0.0))

(fn `Heal`
  (params (`Heal Amount` :type "Float (double-precision)"))
  (returns (`New Health` :type "Float (double-precision)"))
  (return 0.0))

(fn `Init`
  (returns (ReturnValue :type Boolean))
  (bind _returnvalue (`|GetDataTableRow` "/Game/EquipmentForEnemy/DT_Euipment.DT_Euipment" (`self.ID`))
    (:`then`
      (bind _output_get (set `self.Equipment` _returnvalue))
      (bind _returnvalue_2 (`StaticMeshComponent.SetStaticMesh` (`self.StaticMesh`) (`.StaticMesh_48_0BCC07434677176D1138D6B688D5188A` (break `/Game/EquipmentForEnemy/S_Equipment` _output_get))))
      (return _returnvalue_2))))

(fn `On Dead`
  (`PrimitiveComponent.SetSimulatePhysics` (`self.StaticMesh`) true)
  (return))

(fn `Raise Attack`
  (returns (`Now Health` :type "Float (double-precision)") (`Damaged?` :type Boolean))
  (return 0.0 false))

(fn `Return Bonus Value`
  (returns (`Bonus Value` :type "Float (double-precision)"))
  (return 0.0))

(fn `Return Conbat Manager`
  (returns (`Actor Ref` :type "Actor Object Reference"))
  (return null))

(fn `Return Equipment Owner`
  (returns (Actor :type "Actor Object Reference"))
  (return (`self.Master`)))

(fn `Return Fixed Patrol Points`
  (returns (Points :type "Array of Actor Object Reference"))
  (return))

(fn `Return Location`
  (returns (Location :type "Vector Structure"))
  (return (0.0 0.0 0.0)))

(fn `Set Owner`
  (params (Master :type "Actor Object Reference"))
  (set `self.Master` Master)
  (return))

(fn `Take Damage`
  (params (`Damage Info` :type "/Game/Enemy/DamageSystem/S_DamageInfomation Structure"))
  (returns (`Was Damaged?` :type Boolean) (`Now Health` :type "Float (double-precision)"))
  (bind (_damageamount _damagetype _damageresponse _shoulddamageinvincible _canbeblocked _canbeparried _shouldforceinterrupt _element _canaddbuff_ _elementamount _elementdamageamount _buff _instigator _location _toughness) (break `/Game/Enemy/DamageSystem/S_DamageInfomation` `Damage Info`))
  (bind (_was_damaged_ _now_health) (message `/Game/Enemy/DamageSystem/BPI_Damagable.Take Damage` (`self.Master`) (make `/Game/Enemy/DamageSystem/S_DamageInfomation` _damageamount _damagetype _damageresponse _shoulddamageinvincible _canbeblocked _canbeparried _shouldforceinterrupt _element _canaddbuff_ (`self.Element Amount Decrease` _element _elementamount) _elementdamageamount _buff _instigator _location _toughness))) ; 伤害传递，防止打到盔甲上没有给实际actor造成伤害
  (return _was_damaged_ _now_health))

(fn `UserConstructionScript`)