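; AC_Equipment is an enemy equipment component that stores weapons and armor and routes weapon actions.
; On BeginPlay it looks up equipment IDs in DT_Euipment, sorts rows into Weapon and Armor arrays, and messages the owner to add armor resistance.
; Equipment changes are data-only swaps within the same category, with models attached by the armored enemy.
; It also swaps hand weapons, fires weapon abilities and forwards attack-state changes to weapon actors.
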(event `self.ReceiveBeginPlay`
  (`self.Init` (`self.Euipments ID`)))

(fn `Attack State Change`
  (params (`Weapon Index` :type Integer) (Ability :type "/Game/Enemy/Enum/E_HumanAbilities Enum" :default "NewEnumerator0"))
  (bind (_output_id _output_class _output_baseelementresistance _output_basephysicsresistance _output_baseattack _output_isweapon _output_isshield_ _output_shieldbaseresistance _output_ability _output_socket _output_staticmesh _output_actualactor) (break `/Game/EquipmentForEnemy/S_Equipment` (`|GetArrayItem` (`self.Weapon`) `Weapon Index`)))
  (message `/Game/EquipmentForEnemy/BPI_Equipment.Change Attack State` _output_actualactor Ability)
  (return))

(fn `Change Equipment`
  (params (`Put Down Equipment` :type "/Game/EquipmentForEnemy/S_Equipment Structure") (`Put Up Equipment` :type "/Game/EquipmentForEnemy/S_Equipment Structure"))
  (returns (Index :type Integer))
  (bind ((`IsWeapon_34_6B1FD89A4CABEE2FD74D158646982F27` _isweapon)) (break `/Game/EquipmentForEnemy/S_Equipment` `Put Down Equipment`))
  (if (== _isweapon (`.IsWeapon_34_6B1FD89A4CABEE2FD74D158646982F27` (break `/Game/EquipmentForEnemy/S_Equipment` `Put Up Equipment`)))
    (bind _returnvalue (`KismetArrayLibrary.Array_RemoveItem` (select `bool` _isweapon :`false` (`self.Armor`) :`true` (`self.Weapon`)) `Put Down Equipment`))
    (if _returnvalue
      (bind _returnvalue_2 (`KismetArrayLibrary.Array_Add` (select `bool` (`.IsWeapon_34_6B1FD89A4CABEE2FD74D158646982F27` (break `/Game/EquipmentForEnemy/S_Equipment` (`local.Put Up Equipment`))) :`false` (`self.Armor`) :`true` (`self.Weapon`)) (`local.Put Up Equipment`)))
      (return _returnvalue_2)
      (else
        (return -1)))
    (else
      (return -1))))

(fn `Exchange Hand Equipment`
  (`KismetArrayLibrary.Array_Swap` (`self.Weapon`) 1 2)
  (return))

(fn `Init`
  (params (Array :type "Array of Name"))
  (for _array_element Array
    (bind _returnvalue (`|GetDataTableRow` "/Game/EquipmentForEnemy/DT_Euipment.DT_Euipment" _array_element)
      (:`then`
        (if (`.IsWeapon_34_6B1FD89A4CABEE2FD74D158646982F27` (break `/Game/EquipmentForEnemy/S_Equipment` _returnvalue))
          (`KismetArrayLibrary.Array_Add` (`self.Weapon`) _returnvalue)
          (return)
          (else
            (`KismetArrayLibrary.Array_Add` (`self.Armor`) _returnvalue))))))
  (bind _output_get (set `self.Owner` (`self.GetOwner`)))
  (message `/Game/EquipmentForEnemy/BPI_Equipment.Add Armor Resistance` _output_get))

(fn `Use Ability`
  (params (`Use Weapon` :type "/Game/EquipmentForEnemy/S_Equipment Structure"))
  (`/Game/Enemy/BPL_Enemy.Use Ability` (`.Ability_28_DBD6E4D245AD32DA7EFEA28F1A87182A` (break `/Game/EquipmentForEnemy/S_Equipment` `Use Weapon`)) (`self.Owner`))
  (return))