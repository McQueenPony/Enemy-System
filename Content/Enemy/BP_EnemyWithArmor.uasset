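; Enemy Blueprint that wears armor and weapons from its equipment component, spawning each armor piece as an actor attached to a mesh socket.
; Refreshing armor adds physics resistance to the damage system but writes summed element resistance into each piece's map.
; Non-shield weapons add to current attack.
; Equipment changes replace the first armor slot with a data table row, swapping both actor and resistance values.
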(event `self.ReceiveBeginPlay`
  (`self.Init` (`self.Name`)))

(event `self.ReceiveTick`
  (params (DeltaSeconds :type "Float (single-precision)"))
  (`parent.ReceiveTick` DeltaSeconds))

(event `/Game/EquipmentForEnemy/BPI_Equipment.Add Armor Resistance`
  (`self.Refresh Armor`))

(event `/Game/EquipmentForEnemy/BPI_Equipment.Add Weapon Attack`
  (for _array_element (`/Game/EquipmentForEnemy/AC_Equipment.Weapon` (`self.AC_Euipment`))
    (bind (_id _class _baseelementresistance _basephysicsresistance _baseattack _isweapon _isshield_) (break `/Game/EquipmentForEnemy/S_Equipment` _array_element))
    (if (not _isshield_)
      (set `self.Cur Attack` (+ _baseattack (`self.Cur Attack`))))))

(event `Change Equipment and Get DT Row`
  (params (RowName :type Name))
  (bind _returnvalue (`|GetDataTableRow` "/Game/EquipmentForEnemy/DT_Euipment.DT_Euipment" RowName)
    (:`then`
      (`self.Change Equipment` _returnvalue (`|GetArrayItem` (`/Game/EquipmentForEnemy/AC_Equipment.Armor` (`self.AC_Euipment`)))))))

(fn `Change Equipment`
  (params (`Put Up Equipment` :type "/Game/EquipmentForEnemy/S_Equipment Structure") (`Put Down Equipment` :type "/Game/EquipmentForEnemy/S_Equipment Structure"))
  (returns (`Error Reason` :type Name))
  (bind (_id _class _baseelementresistance _basephysicsresistance _baseattack _isweapon _isshield_ _shieldbaseresistance _ability _socket _staticmesh _actualactor) (break `/Game/EquipmentForEnemy/S_Equipment` `Put Down Equipment`))
  (bind _ac_damagesystem (`self.AC_DamageSystem`))
  (bind ((`Class_43_680406A143E7190A5B002693B745AF6E` _class_2) (`Socket_42_85F298F441F9EE30756F73A80A1DD387` _socket_2)) (break `/Game/EquipmentForEnemy/S_Equipment` (`local.Put Up Equipment`)))
  (bind _element_resistance (`/Game/Enemy/DamageSystem/AC_DamageSystem.Element Resistance` (`self.AC_DamageSystem`)))
  (bind (_returnvalue_location _returnvalue_rotation _returnvalue_scale) (`KismetMathLibrary.BreakTransform` (`SceneComponent.GetSocketTransform` (`self.Mesh`) _socket_2 "RTS_World")))
  (`self.K2_DetachFromActor` _actualactor "KeepRelative" "KeepRelative" "KeepRelative")
  (`self.K2_DestroyActor` _actualactor)
  (bind _returnvalue (`|SpawnActorFromClass` _class_2 (`KismetMathLibrary.MakeTransform` _returnvalue_location _returnvalue_rotation _returnvalue_scale) "AlwaysSpawn" "MultiplyWithRoot" self self))
  (bind _returnvalue_2 (`self.K2_AttachToComponent` _returnvalue (`self.Mesh`) _socket_2 "SnapToTarget" "SnapToTarget" "SnapToTarget" true))
  (bind _index (`/Game/EquipmentForEnemy/AC_Equipment.Change Equipment` (`self.AC_Euipment`) (`local.Put Down Equipment`) (`local.Put Up Equipment`)))
  (`/Game/EquipmentForEnemy/BP_EquipmentBase.Set Owner` _returnvalue self)
  (bind _output (`|GetArrayItem` (`/Game/EquipmentForEnemy/AC_Equipment.Armor` (`self.AC_Euipment`)) _index))
  (bind (_id_2 _class_3 _baseelementresistance_2 _basephysicsresistance_2 _baseattack_2 _isweapon_2 _isshield__2 _shieldbaseresistance_2 _ability_2 _socket_3 _staticmesh_2) (break `/Game/EquipmentForEnemy/S_Equipment` _output))
  (`|VariableSetRef` _output (make `/Game/EquipmentForEnemy/S_Equipment` _id_2 _class_3 _baseelementresistance_2 _basephysicsresistance_2 _baseattack_2 _isweapon_2 _isshield__2 _shieldbaseresistance_2 _ability_2 _socket_3 _staticmesh_2 _returnvalue))
  (if _returnvalue_2
    (bind _keys (`BlueprintMapLibrary.Map_Keys` (`/Game/Enemy/DamageSystem/AC_DamageSystem.Element Resistance` (`self.AC_DamageSystem`))))
    (for _array_element _keys
      (`BlueprintMapLibrary.Map_Add` _element_resistance _array_element (+ (- (`BlueprintMapLibrary.Map_Find` _element_resistance _array_element) (`BlueprintMapLibrary.Map_Find` (`.BaseElementResistance_37_C3A7779C48B6D176E6D7B18DD840D915` (break `/Game/EquipmentForEnemy/S_Equipment` (`local.Put Down Equipment`))) _array_element)) (`BlueprintMapLibrary.Map_Find` (`.BaseElementResistance_37_C3A7779C48B6D176E6D7B18DD840D915` (break `/Game/EquipmentForEnemy/S_Equipment` (`local.Put Up Equipment`))) _array_element))))
    (set `/Game/Enemy/DamageSystem/AC_DamageSystem.Physics Resistance` (+ (- (`/Game/Enemy/DamageSystem/AC_DamageSystem.Physics Resistance` _ac_damagesystem) (`.BasePhysicsResistance_38_16CB039643AE55E05DF8BE99FE5AB4FF` (break `/Game/EquipmentForEnemy/S_Equipment` (`local.Put Down Equipment`)))) (`.BasePhysicsResistance_38_16CB039643AE55E05DF8BE99FE5AB4FF` (break `/Game/EquipmentForEnemy/S_Equipment` (`local.Put Up Equipment`)))) _ac_damagesystem)
    (return "None")
    (else
      (return "Can not Attach Actor To Component"))))

(fn `Init`
  (params (RowName :type Name))
  (`parent.Init` RowName))

(fn `On Dead`
  (return))

(fn `Refresh Armor`
  (for (_array_element _array_index) (`/Game/EquipmentForEnemy/AC_Equipment.Armor` (`self.AC_Euipment`))
    (bind (_id _class _baseelementresistance _basephysicsresistance _baseattack _isweapon _isshield_ _shieldbaseresistance _ability _socket) (break `/Game/EquipmentForEnemy/S_Equipment` _array_element))
    (bind (_returnvalue_location _returnvalue_rotation _returnvalue_scale) (`KismetMathLibrary.BreakTransform` (`SceneComponent.GetSocketTransform` (`self.Mesh`) _socket "RTS_World")))
    (bind _returnvalue (`|SpawnActorFromClass` _class (`KismetMathLibrary.MakeTransform` _returnvalue_location _returnvalue_rotation _returnvalue_scale) "AlwaysSpawn" "MultiplyWithRoot" self self))
    (`/Game/EquipmentForEnemy/BP_EquipmentBase.Set Owner` _returnvalue self)
    (bind _output (`|GetArrayItem` (`/Game/EquipmentForEnemy/AC_Equipment.Armor` (`self.AC_Euipment`)) _array_index))
    (bind (_id_2 _class_2 _baseelementresistance_2 _basephysicsresistance_2 _baseattack_2 _isweapon_2 _isshield__2 _shieldbaseresistance_2 _ability_2 _socket_2 _staticmesh) (break `/Game/EquipmentForEnemy/S_Equipment` _output))
    (`|VariableSetRef` _output (make `/Game/EquipmentForEnemy/S_Equipment` _id_2 _class_2 _baseelementresistance_2 _basephysicsresistance_2 _baseattack_2 _isweapon_2 _isshield__2 _shieldbaseresistance_2 _ability_2 _socket_2 _staticmesh _returnvalue))
    (`self.K2_AttachToComponent` _returnvalue (`self.Mesh`) _socket "SnapToTarget" "SnapToTarget" "SnapToTarget" true)
    (set `/Game/Enemy/DamageSystem/AC_DamageSystem.Physics Resistance` (+ _basephysicsresistance (`/Game/Enemy/DamageSystem/AC_DamageSystem.Physics Resistance` (`self.AC_DamageSystem`))) (`self.AC_DamageSystem`))
    (bind _keys (`BlueprintMapLibrary.Map_Keys` _baseelementresistance))
    (for _array_element_2 _keys
      (`BlueprintMapLibrary.Map_Add` _baseelementresistance _array_element_2 (+ (`BlueprintMapLibrary.Map_Find` _baseelementresistance _array_element_2) (`BlueprintMapLibrary.Map_Find` (`/Game/Enemy/DamageSystem/AC_DamageSystem.Element Resistance` (`self.AC_DamageSystem`)) _array_element_2)))))
  (return))

(fn `Return Equipment Owner`
  (returns (Actor :type "Actor Object Reference"))
  (return null))

(fn `UserConstructionScript`
  (`parent.UserConstructionScript`))