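; Enemy damage component that tracks health, toughness and elemental buildup, with invincibility, blocking and death.
; TakeDamage branches to blocked, damaged or ignored, feeding elemental buildup that triggers buffs and resistance-curve reduced physical plus elemental damage.
; Surviving interruptible or force-interrupted hits drain toughness and fire response and knockdown dispatchers.
; A gated Tick regenerates toughness after a retriggerable delay, or immediately during knockdown, clearing KnockDown when full.
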(event `self.ReceiveBeginPlay`)

(event `self.ReceiveTick`
  (params (DeltaSeconds :type "Float (single-precision)"))
  (`/Engine/EditorBlueprintResources/StandardMacros.Gate` false :!label _label
    (:`Exit`
      (bind _new_toughness (`self.Increase Toughness` DeltaSeconds))
      (if (== _new_toughness (`self.Max Toughness`))
        (set `self.Knock Down?` false)))))

(event `Stop Timer`
  (if (`self.Knock Down?`)
    (goto _label :!via `Open`)
    (else
      (`|ExecutionSequence`
        (:`then_0`
          (`KismetSystemLibrary.RetriggerableDelay` 5.0)
          (goto _label :!via `Open`))
        (:`then_1`
          (goto _label :!via `Close`))))))

(fn `Buff Calculate`
  (params (`Cur Element ` :type "/Game/Enemy/DamageSystem/E_ElementType Enum" :default "NewEnumerator0") (`Element Amount` :type "Float (double-precision)") (Creator :type "Actor Object Reference"))
  (bind _completed_ (`/Game/Enemy/BPL_Enemy.Get Buff Last Time` `Cur Element ` (`self.Get Owner`))) ; 获取当前的buff是否生效
  (if _completed_
    (`BlueprintMapLibrary.Map_Add` (`self.Cur Element Amount`) (`local.Cur Element `) (`self.Element Amount Calculate` (`local.Cur Element `) `Element Amount` (`self.Get Cur Element Resisatnce` (`local.Cur Element `))))
    (if (>= (`BlueprintMapLibrary.Map_Find` (`self.Cur Element Amount`) (`local.Cur Element `)) (`BlueprintMapLibrary.Map_Find` (`self.Max Element Amount`) (`local.Cur Element `)))
      (`/Game/Enemy/BPL_Enemy.Add Buff` (`local.Cur Element `) (`local.Creator`) (`self.Get Owner`))
      (`BlueprintMapLibrary.Map_Add` (`self.Cur Element Amount`) (`local.Cur Element `)))
    (return)
    (else
      (return))))

(fn `Damage Reduction Calculate`
  (params (`Damage Amount` :type "Float (double-precision)") (Resistance :type "Float (double-precision)") (`Is Physics Damage?` :type Boolean))
  (returns (`Actual Damage Amount` :type "Float (double-precision)"))
  (return (* `Damage Amount` (- 1.0 (/ Resistance (+ (`KismetMathLibrary.SelectFloat` (`self.Physics Damage Constant`) (`self.Elemental Damage Constant`) `Is Physics Damage?`) Resistance))))))

(fn `Element Amount Calculate`
  (params (Element :type "/Game/Enemy/DamageSystem/E_ElementType Enum (by ref)") (`Element Amount` :type "Float (double-precision)") (`Element Resistance` :type "Float (double-precision)"))
  (returns (`New Element Amount` :type "Float (double-precision)"))
  (bind (_value _returnvalue) (`BlueprintMapLibrary.Map_Find` (`self.Cur Element Amount`) Element))
  (return (`KismetMathLibrary.FClamp` (+ (`KismetMathLibrary.SelectFloat` _value 0.0 _returnvalue) (* `Element Amount` (- 1.0 (/ `Element Resistance` (`self.Element Constant`))))) 0.0 (`BlueprintMapLibrary.Map_Find` (`self.Max Element Amount`) Element))))

(fn `Get Cur Element Resisatnce`
  (params (Element :type "/Game/Enemy/DamageSystem/E_ElementType Enum (by ref)"))
  (returns (Value :type "Float (double-precision)"))
  (return (`BlueprintMapLibrary.Map_Find` (`self.Element Resistance`) Element)))

(fn `Get Owner`
  (returns (ReturnValue :type "Actor Object Reference"))
  (return (`self.GetOwner`)))

(fn `Heal`
  (params (Amount :type "Float (double-precision)"))
  (returns (`New Health` :type "Float (double-precision)"))
  (if (not (`self.Is Dead`))
    (bind _output_get (set `self.Health` (`KismetMathLibrary.FClamp` (+ Amount (`self.Health`)) 0.0 (`self.Max Health`))))
    (return _output_get)
    (else
      (return 0.0))))

(fn `Health Calculate`
  (params (`Physics Damage Amount` :type "Float (double-precision)") (Element :type "/Game/Enemy/DamageSystem/E_ElementType Enum (by ref)") (`Element Damage Amount` :type "Float (double-precision)"))
  (returns (Output_Get :type "Float (double-precision)"))
  (bind _output_get (set `self.Health` (- (`self.Health`) (+ (`self.Damage Reduction Calculate` `Element Damage Amount` (`self.Get Cur Element Resisatnce` Element)) (`self.Damage Reduction Calculate` `Physics Damage Amount` (`self.Physics Resistance`) true)))))
  (return _output_get))

(fn `Increase Toughness`
  (params (`Delta Time` :type "Float (double-precision)"))
  (returns (`New Toughness` :type "Float (double-precision)"))
  (bind _output_get (set `self.Cur Toughness` (`KismetMathLibrary.FClamp` (+ (`self.Cur Toughness`) (* `Delta Time` (`self.Increase Toughness Per Second`))) 0.0 (`self.Max Toughness`))))
  (return _output_get))

(fn `Init`
  (params (`Physics Resistance` :type "Float (double-precision)") (`Element Resistance` :type "Map of /Game/Enemy/DamageSystem/E_ElementType Enum to Float (double-precision)") (Health :type "Float (double-precision)") (`Max Toughness` :type "Float (double-precision)"))
  (set `self.Owner` (`self.GetOwner`))
  (set `self.Physics Resistance` `Physics Resistance`)
  (set `self.Element Resistance` `Element Resistance`)
  (set `self.Health` Health)
  (set `self.Max Health` Health)
  (set `self.Max Toughness` `Max Toughness`)
  (set `self.Cur Toughness` `Max Toughness`)
  (return))

(fn `Sharpening Toughness`
  (params (`Sharpening Toughness` :type "Float (double-precision)"))
  (returns (`Remaining Toughness?` :type Boolean) (`Remaining Toughness` :type "Float (double-precision)"))
  (if (`self.Knock Down?`)
    (return true (`self.Cur Toughness`))
    (else
      (bind _output_get (set `self.Cur Toughness` (`KismetMathLibrary.FClamp` (- (`self.Cur Toughness`) `Sharpening Toughness`) 0.0 (`self.Max Toughness`))))
      (return (> _output_get 0.0) _output_get))))

(fn `Take Damage`
  (params (`Damage Info` :type "/Game/Enemy/DamageSystem/S_DamageInfomation Structure"))
  (returns (`Was Damaged` :type Boolean) (`New Health` :type "Float (double-precision)") (`If Block Return Toughness` :type "Float (double-precision)"))
  (bind ((`DamageAmount_2_A601B9EA4B933BB5EC087998337A0C2A` _damageamount) (`Element_20_297BAD374671704C9D0FC98308CE0696` _element) (`ElementDamageAmount_32_8D2F52D7461E4AE2BCC295B3A1135C2D` _elementdamageamount)) (break `/Game/Enemy/DamageSystem/S_DamageInfomation` (`local.Damage Info`)))
  (bind ((`Element_20_297BAD374671704C9D0FC98308CE0696` _element_2) (`ElementAmount_25_B64637354A71DA824BE700AEAC5FEDF1` _elementamount) (`Instigator_39_CF65D3B04FA7575B2CD9EBAA4EEF8078` _instigator)) (break `/Game/Enemy/DamageSystem/S_DamageInfomation` (`local.Damage Info`)))
  (bind ((`DamageResponse_8_467FFC3A4794C0246500DF9D0D9EDF0D` _damageresponse) (`Toughness_43_D0F2A01144A036F88A0C36A30DEE5608` _toughness)) (break `/Game/Enemy/DamageSystem/S_DamageInfomation` (`local.Damage Info`)))
  (bind ((`CanBeParried_15_FEECDF1148384CEFB84CF780DEAD4C81` _canbeparried) (`Toughness_43_D0F2A01144A036F88A0C36A30DEE5608` _toughness_2)) (break `/Game/Enemy/DamageSystem/S_DamageInfomation` (`local.Damage Info`)))
  (bind ((`ShouldDamageInvincible_11_FF97BBEE4ADD092859EEB6B58FA57EE9` _shoulddamageinvincible) (`CanBeBlocked_13_87BD5DD2455D9CA944C8D7A120B8159F` _canbeblocked)) (break `/Game/Enemy/DamageSystem/S_DamageInfomation` (`local.Damage Info`)))
  (`self.Can Be Damaged` _shoulddamageinvincible _canbeblocked ; 判断伤害是否生效，如何生效
    (:`Block Damage`
      (`self.On Blocked` _canbeparried) ; 伤害被格挡或弹反
      (return false (`self.Health`) _toughness_2))
    (:`Do Damage`
      (`self.Buff Calculate` _element_2 _elementamount _instigator) ; 造成了伤害       异常值计算模块
      (bind _output_get (`self.Health Calculate` _damageamount _element _elementdamageamount)) ; 生命值减少模块
      (if (<= _output_get 0.0)
        (set `self.Is Dead` true)
        (`self.On Death`)
        (elif (or (`self.Is Interruptible`) (`.ShouldForceInterrupt_17_515AD27542E2778D2AFE998D7DD699F8` (break `/Game/Enemy/DamageSystem/S_DamageInfomation` (`local.Damage Info`))))
          (`self.On Damage Response` _damageresponse)
          (bind _remaining_toughness_ (`self.Sharpening Toughness` _toughness))
          (if (not _remaining_toughness_)
            (`self.On Knock Down`))
          (`self.Stop Timer`)))
      (return true (`self.Health`) 0.0))
    (:`No Damage`
      (return false (`self.Health`) 0.0) ; 对象处于无敌帧或其他原因，伤害未生效
    )))