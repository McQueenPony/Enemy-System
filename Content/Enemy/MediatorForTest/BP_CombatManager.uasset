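; Combat manager that limits how many enemies attack one target (the player pawn by default) at once, using the cap the target reports.
; Attack requests join the attacker list or, when it is full, a waiting list, and each requester gets an attack or wait message.
; When an attacker dies, the first waiting one is promoted; when the target dies, all are told to retreat and both lists clear.
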(event `self.ReceiveBeginPlay`
  (`self.Attack Target`
    (:`then`
      _)
    (:`else`
      (set `self.Attack Target` (`GameplayStatics.GetPlayerPawn` 0))))
  (bind _value (message `/Game/Enemy/MediatorForTest/BPI_AttackTarget.Get Max Attackers Count` (`self.Attack Target`)))
  (set `self.Max Attackers Count` _value))

(fn `Engage Waiting Attacker`
  (locals (`Waiting Attacker` :type "Actor Object Reference"))
  (bind _output (`|GetArrayItem` (`self.Waiting Attackers`)))
  (`/Engine/EditorBlueprintResources/StandardMacros.IsValid` _output
    (:`Is Valid`
      (bind _output_get (set `local.Waiting Attacker` _output))
      (`KismetArrayLibrary.Array_RemoveItem` (`self.Waiting Attackers`) _output_get)
      (`KismetArrayLibrary.Array_AddUnique` (`self.Attackers`) _output_get)
      (message `/Game/Enemy/MediatorForTest/BPI_Attacker.Attack` _output_get (`self.Attack Target`)))))

(fn `Handle Attack Request`
  (params (Attacker :type "Actor Object Reference"))
  (returns (`Branch Reason` :type Name))
  (bind _attacker (`local.Attacker`))
  (bind _attacker_2 (`local.Attacker`))
  (if (!= Attacker (`self.Attack Target`))
    (if (< (`KismetArrayLibrary.Array_Length` (`self.Attackers`)) (`self.Max Attackers Count`))
      (`KismetArrayLibrary.Array_AddUnique` (`self.Attackers`) _attacker_2)
      (message `/Game/Enemy/MediatorForTest/BPI_Attacker.Attack` _attacker_2 (`self.Attack Target`))
      (return "Attack")
      (else
        (`KismetArrayLibrary.Array_AddUnique` (`self.Waiting Attackers`) _attacker)
        (message `/Game/Enemy/MediatorForTest/BPI_Attacker.Wait` _attacker (`self.Attack Target`))
        (return "Wait")))
    (else
      (return "Is Attack Target"))))

(fn `Handle Death`
  (params (`Actor Ref` :type "Actor Object Reference"))
  (returns (`Branch Resault` :type Name))
  (if (== `Actor Ref` (`self.Attack Target`))
    (`KismetArrayLibrary.Array_Append` (`self.Attackers`) (`self.Waiting Attackers`))
    (for _array_element (`self.Attackers`)
      (message `/Game/Enemy/MediatorForTest/BPI_Attacker.Retreat` _array_element))
    (`KismetArrayLibrary.Array_Clear` (`self.Attackers`))
    (`KismetArrayLibrary.Array_Clear` (`self.Waiting Attackers`))
    (return "Attack Target Done")
    (elif (`KismetArrayLibrary.Array_Contains` (`self.Attackers`) (`local.Actor Ref`))
      (`KismetArrayLibrary.Array_RemoveItem` (`self.Attackers`) (`local.Actor Ref`))
      (`self.Engage Waiting Attacker`)
      (return "Attacker Done")
      (elif (`KismetArrayLibrary.Array_Contains` (`self.Waiting Attackers`) (`local.Actor Ref`))
        (`KismetArrayLibrary.Array_RemoveItem` (`self.Waiting Attackers`) (`local.Actor Ref`))
        (return "Waiting Attacker Done")
        (else
          (return "Do Not Have Waiting Attackers"))))))

(fn `On Attack Request`
  (params (attacker :type "Actor Object Reference"))
  (returns (`Branch Reason` :type Name))
  (bind _branch_reason (`self.Handle Attack Request` attacker))
  (return _branch_reason))

(fn `On Requester Death`
  (params (`Actor Ref` :type "Actor Object Reference"))
  (returns (`Branch Reason` :type Name))
  (bind _branch_resault (`self.Handle Death` `Actor Ref`))
  (return _branch_resault))

(fn `UserConstructionScript`
  (message `/Game/Enemy/MediatorForTest/BPI_AttackTarget.Get Max Attackers Count` (`self.Attack Target`)))