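; Base enemy Blueprint that loads its stats from DT_Enemy by row name and delegates health, resistances, toughness and buffs to damage and buff components.
; TakeDamage reports to AI damage sensing and triggers knockdown when toughness runs out; death ragdolls the mesh, rolls weighted loot drops and notifies CombatManager.
; Attack/Wait events toggle a blackboard flag for group attack scheduling, while player-action reactions are print-only stubs.
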(event `self.ReceiveTick`
  (params (DeltaSeconds :type "Float (single-precision)")))

(event `/Game/Enemy/DamageSystem/BPI_Damagable.Add Buff`
  (params (ID :type Name) (`Create Actor` :type "Actor Object Reference") (`Target Actor` :type "Actor Object Reference"))
  (`/Game/BUFF/AC_BuffHandler.Add Buff` (`self.AC_BuffHandler`) ID `Create Actor` `Target Actor`))

(event `self.ReceiveBeginPlay`
  (`self.Init` (`self.Name`)))

(event `On Death`
  (bind (_returnvalue_location _returnvalue_rotation) (`KismetMathLibrary.BreakTransform` (`self.GetTransform`)))
  (`KismetSystemLibrary.PrintString` "DEAD")
  (message `/Game/EquipmentForEnemy/BPI_Equipment.On Dead` (`self.GetAttachedActors` true true))
  (`PrimitiveComponent.SetSimulatePhysics` (`self.Mesh`) true)
  (`PrimitiveComponent.SetCollisionEnabled` (`self.Mesh`) "QueryAndPhysics")
  (`BlackboardComponent.SetValueAsBool` (`AIBlueprintHelperLibrary.GetBlackboard` (`self.AI Controller`)) "Dead？" true)
  (for _array_element (`.GivenGoods_39_B911A59643C3B209F7E8AC9A5C88826A` (break `/Game/Enemy/Structure/S_EnemyBase` (`self.Enemy Base`)))
    (bind (_class _fallingprobability _failingnumber) (break `/Game/Enemy/GoodsSystem/S_Goods` _array_element))
    (if (`KismetMathLibrary.RandomBoolWithWeight` _fallingprobability)
      (bind _returnvalue (`|SpawnActorFromClass` "/Game/Enemy/GoodsSystem/BP_Goods.BP_Goods_C" (`KismetMathLibrary.MakeTransform` _returnvalue_location _returnvalue_rotation) "AlwaysSpawn" "MultiplyWithRoot" null null))
      (`/Game/Enemy/GoodsSystem/BP_Goods.Init` _returnvalue _class _fallingprobability _failingnumber)))
  (message `/Game/Enemy/MediatorForTest/BPI_Mediator.On Requester Death` (`self.Combat Manager`) self))

(event `On Blocked`
  (params (`Can Be Parried` :type Boolean))
  (`KismetSystemLibrary.PrintString` "BLOCKED"))

(event `Damage Response`
  (params (Response :type "/Game/Enemy/DamageSystem/E_DamageResponse Enum" :default "NewEnumerator0"))
  (if (`|EnumInequality` Response "NewEnumerator0")
    (`KismetSystemLibrary.PrintString` (`|GetEnumeratorNameAsString` Response))))

(event `Be Knock Down`
  (set `self.Cur State` "NewEnumerator8")
  (`KismetSystemLibrary.PrintString` "Knock Down")
  (set `/Game/Enemy/DamageSystem/AC_DamageSystem.Knock Down?` true (`self.AC_DamageSystem`)))

(event `/Game/Enemy/MediatorForTest/BPI_Attacker.Attack`
  (params (`Attack Target` :type "Actor Object Reference"))
  ;[1 1 1] 集群敌人调度
  (set `self.Can Attack?` true)
  (`BlackboardComponent.SetValueAsBool` (`AIBlueprintHelperLibrary.GetBlackboard` (`self.AI Controller`)) "Can Attack?" true))

(event `/Game/Enemy/MediatorForTest/BPI_Attacker.Wait`
  (params (`Attack Target` :type "Actor Object Reference"))
  ;[1 1 1] 集群敌人调度
  (set `self.Can Attack?` false)
  (`BlackboardComponent.SetValueAsBool` (`AIBlueprintHelperLibrary.GetBlackboard` (`self.AI Controller`)) "Can Attack?" false))

(event `/Game/Enemy/DamageSystem/BPI_Damagable.Player Healing`
  ;[1 1 1] 读指令
  (`KismetSystemLibrary.PrintString` "Player Is Healing!!!!!!"))

(event `/Game/Enemy/DamageSystem/BPI_Damagable.Player Attacking`
  ;[1 1 1] 读指令
  (`KismetSystemLibrary.PrintString` "Player Is Attacking!!!!!!"))

(fn `Begin to Attack`
  (returns (`Now Health` :type "Float (double-precision)") (`Damaged?` :type Boolean))
  (return 0.0 false))

(fn `Get Buff Handler`
  (returns (`AC_Buff Handler` :type "/Game/BUFF/AC_BuffHandler Object Reference"))
  (return (`self.AC_BuffHandler`)))

(fn `Get Current Health`
  (returns (Health :type "Float (double-precision)"))
  (return (`/Game/Enemy/DamageSystem/AC_DamageSystem.Health` (`self.AC_DamageSystem`))))

(fn `Get Current Toughness`
  (returns (Value :type "Float (double-precision)"))
  (return (`/Game/Enemy/DamageSystem/AC_DamageSystem.Cur Toughness` (`self.AC_DamageSystem`))))

(fn `Get Max Health`
  (returns (`Max Health` :type "Float (double-precision)"))
  (return (`/Game/Enemy/DamageSystem/AC_DamageSystem.Max Health` (`self.AC_DamageSystem`))))

(fn `Get Max Toughness`
  (returns (Value :type "Float (double-precision)"))
  (return (`/Game/Enemy/DamageSystem/AC_DamageSystem.Max Toughness` (`self.AC_DamageSystem`))))

(fn `Heal`
  (params (`Heal Amount` :type "Float (double-precision)"))
  (returns (`New Health` :type "Float (double-precision)"))
  (bind _new_health (`/Game/Enemy/DamageSystem/AC_DamageSystem.Heal` (`self.AC_DamageSystem`) `Heal Amount`))
  (return _new_health))

(fn `Init`
  (params (RowName :type Name))
  (bind _returnvalue (`|GetDataTableRow` "/Game/Enemy/DT_Enemy.DT_Enemy" RowName)
    (:`then`
      (bind _output_get (set `self.Enemy Base` (make `/Game/Enemy/Structure/S_EnemyBase` (break `/Game/Enemy/Structure/S_EnemyBase` _returnvalue) (`.Resistance_7_7949C14C4B30A3A393064E9057C14287` (break `/Game/Enemy/Structure/S_EnemyBase` _returnvalue)) (`.CanReborn?_10_C59452564201599EE74535BE579BE845` (break `/Game/Enemy/Structure/S_EnemyBase` _returnvalue)) (`.IsHuman?_12_E4FE83BA41229F3D98B67982D5818DD8` (break `/Game/Enemy/Structure/S_EnemyBase` _returnvalue)) (`.Abilities_19_5032D486457640382AA87785F6B51260` (break `/Game/Enemy/Structure/S_EnemyBase` _returnvalue)) (`.Weapon_21_19D45257490A308D30BC849D95AB18C6` (break `/Game/Enemy/Structure/S_EnemyBase` _returnvalue)) (`.GivenGoods_39_B911A59643C3B209F7E8AC9A5C88826A` (break `/Game/Enemy/Structure/S_EnemyBase` _returnvalue)) (`self.Regional Bonus Value`) (`self.Cur State`) (`self.Begin Target`) (`.Toughness_42_FBB446E34B0FE802C921EEA326587E1B` (break `/Game/Enemy/Structure/S_EnemyBase` _returnvalue)))))
      (bind (_magic _fire _freeze _poison _death _thunder) (break `/Game/Enemy/Structure/S_Resistance` (`.Resistance_7_7949C14C4B30A3A393064E9057C14287` (break `/Game/Enemy/Structure/S_EnemyBase` _returnvalue))))
      (bind (_basehealth _resistance _canreborn_ _ishuman_ _abilities _weapon _givengoods _regionalbonusvalue) (break `/Game/Enemy/Structure/S_EnemyBase` _output_get))
      (`/Game/Enemy/DamageSystem/AC_DamageSystem.Init` (`self.AC_DamageSystem`) (`self.Physics Resistance`) (`|MakeMap` "NewEnumerator1" _magic "NewEnumerator2" _fire "NewEnumerator3" _freeze "NewEnumerator4" _poison "NewEnumerator5" _death "NewEnumerator7" _thunder :!type "/Game/Enemy/DamageSystem/E_ElementType Enum") (* _basehealth _regionalbonusvalue) (`.Toughness_42_FBB446E34B0FE802C921EEA326587E1B` (break `/Game/Enemy/Structure/S_EnemyBase` _returnvalue))))
    (:`RowNotFound`
      _))
  (set `self.AI Controller` (`AIBlueprintHelperLibrary.GetAIController` self))
  (return))

(fn `Raise Attack`
  (returns (`Now Health` :type "Float (double-precision)") (`Damaged?` :type Boolean))
  (bind (_now_health _damaged_) (`self.Begin to Attack`))
  (return _now_health _damaged_))

(fn `Return Bonus Value`
  (returns (`Bonus Value` :type "Float (double-precision)"))
  (return (`.RegionalBonusValue_30_F53E3DE34298B2BC48C30E8375BF65FC` (break `/Game/Enemy/Structure/S_EnemyBase` (`self.Enemy Base`)))))

(fn `Return Conbat Manager`
  (returns (`Actor Ref` :type "Actor Object Reference"))
  (return (`self.Combat Manager`)))

(fn `Return Fixed Patrol Points`
  (returns (Points :type "Array of Actor Object Reference"))
  (return (`self.Fixed Patrol Points`)))

(fn `Return Location`
  (returns (Location :type "Vector Structure"))
  (return (`self.K2_GetActorLocation`)))

(fn `Spawn Projectile`
  (params (Class :type "/Game/Projectile/E_Projectile Enum" :default "NewEnumerator0") (SpawnTransform :type "Transform Structure") (Speed :type "Float (double-precision)") (Gravity :type "Float (double-precision)"))
  (bind _returnvalue (`|SpawnActorFromClass` (select `/Game/Projectile/E_Projectile` Class :`NewEnumerator0` "/Game/Projectile/BP_FireBall.BP_FireBall_C" :`NewEnumerator1` "/Game/Projectile/BP_Ice.BP_Ice_C" :`NewEnumerator2` "/Game/Projectile/BP_Arrow.BP_Arrow_C" :!type "/Game/Projectile/BP_ProjectileBase Class Reference") SpawnTransform "AlwaysSpawn" "MultiplyWithRoot" self Speed Gravity self))
  (`PrimitiveComponent.IgnoreActorWhenMoving` (`self.CapsuleComponent`) _returnvalue true)
  (return))

(fn `Take Damage`
  (params (`Damage Info` :type "/Game/Enemy/DamageSystem/S_DamageInfomation Structure"))
  (returns (`Was Damaged?` :type Boolean) (`Now Health` :type "Float (double-precision)"))
  (bind (_damageamount _damagetype _damageresponse _shoulddamageinvincible _canbeblocked _canbeparried _shouldforceinterrupt _element _canaddbuff_ _elementamount _elementdamageamount _buff _instigator _location) (break `/Game/Enemy/DamageSystem/S_DamageInfomation` `Damage Info`))
  (bind (_bblockinghit _binitialoverlap _time _distance _location_2 _impactpoint) (`GameplayStatics.BreakHitResult` _location))
  (`AISense_Damage.ReportDamageEvent` self null _damageamount _location_2 _impactpoint)
  (bind (_was_damaged _new_health _if_block_return_toughness) (`/Game/Enemy/DamageSystem/AC_DamageSystem.Take Damage` (`self.AC_DamageSystem`) `Damage Info`))
  (if (not (== _if_block_return_toughness 0.0))
    (bind _remaining_toughness_ (`/Game/Enemy/DamageSystem/AC_DamageSystem.Sharpening Toughness` (`self.AC_DamageSystem`) _if_block_return_toughness))
    (if (not _remaining_toughness_)
      (`self.Be Knock Down`)))
  (return _was_damaged _new_health))

(fn `UserConstructionScript`
  (bind _ac_damagesystem (`self.AC_DamageSystem`))
  (add `/Game/Enemy/DamageSystem/AC_DamageSystem.On Death` _ac_damagesystem (`|CreateDelegate` :!event `On Death`))
  (add `/Game/Enemy/DamageSystem/AC_DamageSystem.On Blocked` _ac_damagesystem (`|CreateDelegate` :!event `On Blocked`))
  (add `/Game/Enemy/DamageSystem/AC_DamageSystem.On Damage Response` _ac_damagesystem (`|CreateDelegate` :!event `Damage Response`))
  (add `/Game/Enemy/DamageSystem/AC_DamageSystem.On Knock Down` _ac_damagesystem (`|CreateDelegate` :!event `Be Knock Down`)))