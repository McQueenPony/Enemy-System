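; Base projectile actor that flies at a set speed and gravity, optionally homing on a target, and delivers damage on impact.
; Construction configures the movement component; BeginPlay ignores the owner for collision and aims velocity at any valid target.
; A box hit fires the impact dispatcher, plays sound and emitter effects, then destroys the projectile.
; ProjectileImpact sends a damage-info message to an actor, scaling damage and element amounts by the owner's bonus value.
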(event `self.ReceiveBeginPlay`
  (`PrimitiveComponent.IgnoreActorWhenMoving` (`self.Box`) (`self.GetOwner`) true)
  (`self.Target`
    (:`then`
      (`self.Rotate to Target`))
    (:`else`)))

(event `Rotate to Target`
  (set `MovementComponent.Velocity` (* (`KismetMathLibrary.GetDirectionUnitVector` (`self.K2_GetActorLocation`) (`self.K2_GetActorLocation` (`self.Target`))) (`self.Speed`)) (`self.ProjectileMovement`)))

(event `self.Box.OnComponentHit`
  (params (HitComponent :type "PrimitiveComponent Object Reference") (OtherActor :type "Actor Object Reference") (OtherComp :type "PrimitiveComponent Object Reference") (NormalImpulse :type "Vector Structure") (Hit :type "HitResult Structure (by ref)"))
  (`self.On Projectile Impact` OtherActor Hit)
  (`GameplayStatics.PlaySoundAtLocation` (`self.Sound`) (`self.K2_GetActorLocation`) (struct) 1.0 1.0 0.0 null null null null)
  (`GameplayStatics.SpawnEmitterAtLocation` (`self.Emitter Template`) (`self.K2_GetActorLocation`))
  (`self.K2_DestroyActor`))

(fn `Projectile Impact`
  (params (Actor :type "Actor Object Reference") (Hit :type "HitResult Structure"))
  (bind (_damage_info_damageamount _damage_info_damagetype _damage_info_damageresponse _damage_info_shoulddamageinvincible _damage_info_canbeblocked _damage_info_canbeparried _damage_info_shouldforceinterrupt _damage_info_element _damage_info_canaddbuff_ _damage_info_elementamount _damage_info_elementdamageamount _damage_info_buff _damage_info_instigator) (break `/Game/Enemy/DamageSystem/S_DamageInfomation` (`self.Damage Info`)))
  (bind _bonus_value (message `/Game/Enemy/DamageSystem/BPI_Damagable.Return Bonus Value` (`self.GetOwner`)))
  (message `/Game/Enemy/DamageSystem/BPI_Damagable.Take Damage` Actor (make `/Game/Enemy/DamageSystem/S_DamageInfomation` (* _bonus_value _damage_info_damageamount) _damage_info_damagetype _damage_info_damageresponse _damage_info_shoulddamageinvincible _damage_info_canbeblocked _damage_info_canbeparried _damage_info_shouldforceinterrupt _damage_info_element _damage_info_canaddbuff_ (* _bonus_value _damage_info_elementamount) (* _bonus_value _damage_info_elementdamageamount) _damage_info_buff _damage_info_instigator Hit)))

(fn `UserConstructionScript`
  (bind _projectilemovement (`self.ProjectileMovement`))
  (set `ProjectileMovementComponent.InitialSpeed` (`self.Speed`) _projectilemovement)
  (set `ProjectileMovementComponent.MaxSpeed` (`self.Speed`) _projectilemovement)
  (set `ProjectileMovementComponent.ProjectileGravityScale` (`self.Gravity`) _projectilemovement)
  (bind _target (`self.Target`)
    (:`then`
      (set `ProjectileMovementComponent.bIsHomingProjectile` (`self.Homing`) _projectilemovement)
      (set `ProjectileMovementComponent.HomingTargetComponent` (`Actor.RootComponent` _target) _projectilemovement)
      (add `self.On Projectile Impact` (`|CreateDelegate` :!event `Projectile Impact`)))
    (:`else`)))